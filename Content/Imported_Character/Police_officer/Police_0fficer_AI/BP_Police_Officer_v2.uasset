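; Police officer AI character that shoots pawns ahead of it with a pistol and can be killed by damage.
; Fire checks the blackboard's TargetNear? flag, then sphere-traces forward to damage the hit pawn and spawns impact and muzzle effects.
; A FirstTime flag, re-armed on Tick while no target is near, skips the animation-sync delay on the opening shot.
; Incoming damage lowers Health, prints it, spawns an explosion, and destroys the actor only at exactly zero.
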(event EventBeginPlay)

(event Collision|EventActorBeginOverlap
  (params (OtherActor :type Actor%20Object%20Reference)))

(event EventFire
  (bind _returnvalue (Transformation|GetActorLocation))
  (bind _pistol (Variables|Default|GetPistol))
  (bind _returnvalue_2 (Transformation|GetSocketTransform _pistol "muzzle" "RTS_World"))
  ;[1 1 1] Fire
  (if (Variables|Default|GetFirstTime?)
    _
    (else
      (Utilities|FlowControl|Delay 1.18)))
  (if (ScalableFloat|GetValueasBool (AI|GetBlackboard 0) (Utilities|Name|MakeLiteralName "TargetNear?"))
    (Utilities|FlowControl|Sequence
      (:then_0
        (bind (_outhit _returnvalue_3) (Collision|SphereTraceForObjects _returnvalue (+ _returnvalue (* (Math|Vector|GetForwardVector (Transformation|GetActorRotation)) 5e+03)) 25.0 (Utilities|Array|MakeArray "ObjectTypeQuery3") false 0 "ForDuration"))
        (if _returnvalue_3
          (Effects|SpawnEmitteratLocation 0 (.ImpactPoint (Collision|BreakHitResult _outhit)) (Math|Rotator|MakeRotfromX (.Normal (Collision|BreakHitResult _outhit))) "0.300000,0.300000,0.300000" true "AutoRelease")
          (Game|Damage|ApplyDamage (.HitActor (Collision|BreakHitResult _outhit)) 8.0 0 0)
          (Variables|Default|SetFirstTime? false)))
      (:then_1
        (Effects|SpawnEmitterAttached 0 (Variables|Default|GetPistol) "muzzle" (.location _returnvalue_2) (.rotation _returnvalue_2) "0.100000,0.100000,0.100000" "KeepWorldPosition" true "AutoRelease")))))

(event Game|Damage|EventAnyDamage
  (params (Damage :type Float%20%28single-precision%29) (DamageType :type Damage%20Type%20Object%20Reference) (InstigatedBy :type Controller%20Object%20Reference) (DamageCauser :type Actor%20Object%20Reference))
  ;[1 1 1] Taking Damage
  (bind _output_get (Variables|Default|SetHealth (- (Variables|Default|GetHealth) Damage)))
  (Development|PrintString (Utilities|String|ToString(Float) _output_get) true true "(R=1.000000,G=0.000000,B=0.981017,A=1.000000)")
  (Effects|SpawnEmitteratLocation "/Game/StarterContent/Particles/P_Explosion.P_Explosion" (Transformation|GetActorLocation))
  (if (== (Variables|Default|GetHealth) 0.0)
    (Actor|DestroyActor)))

(event EventTick
  (params (DeltaSeconds :type Float%20%28single-precision%29))
  ;[1 1 1] First Time Fire (Animation synchronization)
  (if (not (ScalableFloat|GetValueasBool (AI|GetBlackboard 0) (Utilities|Name|MakeLiteralName "TargetNear?")))
    (Variables|Default|SetFirstTime? true)))

(fn ConstructionScript)