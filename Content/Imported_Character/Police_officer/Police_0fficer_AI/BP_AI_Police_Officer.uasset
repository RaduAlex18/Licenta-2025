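; AI controller for the police officer that runs its behavior tree on BeginPlay and feeds it perception results.
; Sight updates the seen flag and, on success, clears the heard flag and stores the sensed actor as target in the blackboard.
; Hearing sets the heard flag and target only when nothing is seen, saving the noise location in a controller variable.
; Debug strings print on perception updates.
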(event OnTargetPerceptionUpdated(AIPerception)
  (params (Actor :type Actor%20Object%20Reference) (Stimulus :type AI%20Stimulus%20Structure))
  (bind (_stimuluslocation _bsuccessfullysensed) (Utilities|Struct|BreakAIStimulus Stimulus))
  (bind _returnvalue (Class|AIPerceptionSystem|GetSenseClassforStimulus Stimulus))
  (if (== _returnvalue "/Script/AIModule.AISense_Sight")
    (Development|PrintString "Te vad")
    (if _bsuccessfullysensed
      (AI|Components|Blackboard|SetValueasBool (AI|GetBlackboard 0) (Utilities|Name|MakeLiteralName "TargetHeard?") false)
      ;[0 1 0.3174] The AI ​​sees the player
      (AI|Components|Blackboard|SetValueasBool (AI|GetBlackboard 0) (Utilities|Name|MakeLiteralName "TargetSeen?") true)
      (AI|Components|Blackboard|SetValueasObject (AI|GetBlackboard 0) (Utilities|Name|MakeLiteralName "targetPlayer") Actor)
      (else
        ;[1 0 0.299] The AI ​​doesn't see the player
        (AI|Components|Blackboard|SetValueasBool (AI|GetBlackboard 0) (Utilities|Name|MakeLiteralName "TargetSeen?") false)))
    (elif (== _returnvalue "/Script/AIModule.AISense_Hearing")
      (Development|PrintString "Te aud")
      (if _bsuccessfullysensed
        (if (not (ScalableFloat|GetValueasBool (AI|GetBlackboard 0) (Utilities|Name|MakeLiteralName "TargetSeen?")))
          (AI|Components|Blackboard|SetValueasBool (AI|GetBlackboard 0) (Utilities|Name|MakeLiteralName "TargetHeard?") true)
          (AI|Components|Blackboard|SetValueasObject (AI|GetBlackboard 0) (Utilities|Name|MakeLiteralName "targetPlayer") Actor)
          (Variables|Default|SetLocationsPlayer _stimuluslocation)
          (Development|PrintString (Utilities|String|ToString(Vector) _stimuluslocation))
          (else
            (AI|Components|Blackboard|SetValueasBool (AI|GetBlackboard 0) (Utilities|Name|MakeLiteralName "TargetHeard?") false :!label _label)))
        (else
          (goto _label))))))

(event EventBeginPlay
  (AI|RunBehaviorTree "/Game/Imported_Character/Police_officer/Police_0fficer_AI/BT_Police_Officer_AI.BT_Police_Officer_AI"))

(fn ConstructionScript)